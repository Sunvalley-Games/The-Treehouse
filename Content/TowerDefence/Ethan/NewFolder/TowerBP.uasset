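; Tower defence tower that snaps onto a Platform beneath it and fires projectiles at enemies.
; On BeginPlay, a downward multi-line trace finds the platform, moves the tower to it, sets Occupied and caches the EnemyAISpawner.
; Sphere overlap makes the newest entering EnemyAI01 the current target.
; A looping one-second timer spawns a Projectile aimed at that target while valid and passes it the spawner.
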(event OnComponentBeginOverlap(Sphere)
  (params (OverlappedComponent :type Primitive%20Component%20Object%20Reference) (OtherActor :type Actor%20Object%20Reference) (OtherComp :type Primitive%20Component%20Object%20Reference) (OtherBodyIndex :type Integer) (bFromSweep :type Boolean) (SweepResult :type Hit%20Result%20Structure%20%28by%20ref%29))
  (Utilities|Casting|CastToEnemyAI01 OtherActor)
  (Variables|Default|SetCurrentTarget OtherActor))

(event Custom|Fire
  (bind _currenttarget (Variables|Default|GetCurrentTarget))
  (if (Utilities|IsValid _currenttarget)
    (bind _asenemy_ai01 (Utilities|Casting|CastToEnemyAI01 _currenttarget))
    (bind _returnvalue (Game|SpawnActorfromClass "/Game/TowerDefence/Ethan/NewFolder/Projectile.Projectile_C" (Transformation|GetActorTransform) "AlwaysSpawn" 0 _asenemy_ai01 0))
    (bind _asprojectile (Utilities|Casting|CastToProjectile _returnvalue))
    (Default|AssignSpawner _asprojectile (Variables|Default|GetEnemySpawner))))

(event EventBeginPlay
  (bind _returnvalue (Transformation|GetActorTransform))
  (Utilities|Time|SetTimerbyEvent (delegate Custom|Fire) 1.0 true)
  (bind (_outhits _returnvalue_2) (Class|KismetSystemLibrary|LineTraceMultiforObjects (.location _returnvalue) (- (.location _returnvalue) "0,0.000000,1000000.000000") (Utilities|Array|MakeArray "ObjectTypeQuery2") false 0 "None" true))
  (if _returnvalue_2
    (for _array_element _outhits
      (Development|PrintString (Utilities|GetDisplayName (.HitActor (Collision|BreakHitResult _array_element))))
      (bind _asplatform (Utilities|Casting|CastToPlatform (.HitActor (Collision|BreakHitResult _array_element)))
        (:then
          (if (not (Variables|Default|GetOccupied))
            (Variables|Default|SetOccupied true)
            (Transformation|SetActorLocation self (Transformation|GetActorLocation _asplatform) false false)
            (bind _returnvalue_3 (Actor|GetActorOfClass "/Game/TowerDefence/Connor/EnemyAISpawner.EnemyAISpawner_C"))
            (Variables|Default|SetEnemySpawner _returnvalue_3)))
        (:CastFailed
          (Development|PrintString "Invalid Target" true true "(R=1.000000,G=0.000000,B=0.079151,A=1.000000)"))))))

(event Collision|EventActorBeginOverlap
  (params (OtherActor :type Actor%20Object%20Reference)))

(event EventTick
  (params (DeltaSeconds :type Float%20%28single-precision%29)))

(fn ConstructionScript
  (Utilities|Array|Add (Variables|Default|GetActorList) self))