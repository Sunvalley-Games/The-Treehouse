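; VR push button that, when fully pressed, either starts the game through EnemyAISpawner or opens a configured level, depending on StartLevel.
; Overlapping BP_MotionController begins tracking; Tick projects hand movement onto the button's up vector to set clamped travel.
; Full travel raises the dynamic material's glow and fires FullyPress, repeatedly while held in StartLevel mode.
; Releasing interpolates the button back, then resets the glow.
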(event OnComponentBeginOverlap(VR_button_Button)
  (params (OverlappedComponent :type Primitive%20Component%20Object%20Reference) (OtherActor :type Actor%20Object%20Reference) (OtherComp :type Primitive%20Component%20Object%20Reference) (OtherBodyIndex :type Integer) (bFromSweep :type Boolean) (SweepResult :type Hit%20Result%20Structure%20%28by%20ref%29))
  (if (and (not (Variables|Default|GetTracking)) (not (Variables|Default|GetButtonReturning)))
    (bind _asbp_motion_controller (Utilities|Casting|CastToBP_MotionController OtherActor))
    (Variables|Default|SetVr_hand (Variables|/Game/VirtualRealityBP/Blueprints/BP_MotionController.BP_MotionController_C|GetMotionController _asbp_motion_controller))
    (Variables|Default|SetTracking true)
    (Variables|Default|SetHandLocation (Transformation|GetWorldLocation (Variables|Default|GetVr_hand)))
    (Variables|Default|SetButtonLocation (Transformation|GetWorldLocation (Variables|Default|GetVR_button_Button)))))

(event OnComponentEndOverlap(VR_button_Button)
  (params (OverlappedComponent :type Primitive%20Component%20Object%20Reference) (OtherActor :type Actor%20Object%20Reference) (OtherComp :type Primitive%20Component%20Object%20Reference) (OtherBodyIndex :type Integer))
  (bind _asbp_motion_controller (Utilities|Casting|CastToBP_MotionController OtherActor))
  (if (== (Variables|Default|GetVr_hand) (Variables|/Game/VirtualRealityBP/Blueprints/BP_MotionController.BP_MotionController_C|GetMotionController _asbp_motion_controller))
    (Variables|Default|SetTracking false)
    (Variables|Default|SetButtonReturning true)))

(event Custom|FullyPress
  (Rendering|Material|SetScalarParameterValue (Variables|Default|GetMaterialButton) "Glow" (Variables|Default|GetGlowIntenseValue) :!class /Script/Engine.MaterialInstanceDynamic)
  (if (Variables|Default|GetStartLevel)
    (bind _returnvalue (Actor|GetActorOfClass "/Game/TowerDefence/Connor/EnemyAISpawner.EnemyAISpawner_C"))
    (bind _asenemy_aispawner (Utilities|Casting|CastToEnemyAISpawner _returnvalue)
      (:then
        (Default|StartGame _asenemy_aispawner))
      (:CastFailed
        (Development|PrintString "Cast Failed" true true "(R=1.000000,G=0.000000,B=0.086574,A=1.000000)")))
    (else
      (Variables|Default|SetTracking false)
      (Variables|Default|SetButtonReturning true)
      (Game|OpenLevel(byName) (Variables|Default|GetLevelToLoad)))))

(event EventTick
  (params (DeltaSeconds :type Float%20%28single-precision%29))
  (bind _vr_button_button (Variables|Default|GetVR_button_Button))
  (if (Variables|Default|GetTracking)
    (Variables|Default|SetCurrentTravel (Math|Float|Clamp(Float) (Math|Float|Absolute(Float) (Math|Vector|VectorLength (Math|Vector|ProjectVectorontoVector (- (Transformation|GetWorldLocation (Variables|Default|GetVr_hand)) (Variables|Default|GetHandLocation)) (Math|Vector|GetUpVector (Variables|Default|GetVR_button_Button))))) 0.0 (Variables|Default|GetMaximum_tra)))
    (bind _output_get (Variables|Default|SetButtonCurrentLocaiton (- (Variables|Default|GetButtonLocation) (* (Math|Vector|GetUpVector _vr_button_button) (Variables|Default|GetCurrentTravel)))))
    (Transformation|SetWorldLocation _vr_button_button _output_get false false)
    (if (>= (Variables|Default|GetCurrentTravel) (Variables|Default|GetMaximum_tra))
      (CallFunction|FullyPress))
    (elif (Variables|Default|GetButtonReturning)
      (bind _output_get_2 (Variables|Default|SetButtonCurrentLocaiton (Math|Interpolation|VInterpTo (Variables|Default|GetButtonCurrentLocaiton) (Variables|Default|GetButtonLocation) (Utilities|Time|GetWorldDeltaSeconds) (Variables|Default|GetButtonReturnSpeed))))
      (Transformation|SetWorldLocation (Variables|Default|GetVR_button_Button) _output_get_2 false false)
      (if (Class|KismetMathLibrary|EqualExactlyVectorVector (Variables|Default|GetButtonCurrentLocaiton) (Variables|Default|GetButtonLocation))
        (Variables|Default|SetButtonReturning false)
        (Rendering|Material|SetScalarParameterValue (Variables|Default|GetMaterialButton) "Glow" 1.0 :!class /Script/Engine.MaterialInstanceDynamic)))))

(event EventBeginPlay
  (bind _returnvalue (Rendering|Material|CreateDynamicMaterialInstance (Variables|Default|GetVR_button_Button) 0 "/Game/Labyrinth/Materials/Button.Button" "None" :!class /Script/Engine.PrimitiveComponent))
  (Variables|Default|SetMaterialButton _returnvalue))

(fn ConstructionScript)