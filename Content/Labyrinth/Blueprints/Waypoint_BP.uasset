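; Waypoint actor for the labyrinth that plays a sound until the first-person player reaches it.
; On BeginPlay it caches the player character and the WaypointManagement_BP instance; PlayMusic starts its SoundSource.
; The first player overlap fades out and stops the sound, hides the actor and tells the manager to start the next waypoint.
; An unconnected LocomotionPawn_Final cast remains unused.
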(event OnComponentBeginOverlap(Collider)
  (params (OverlappedComponent :type Primitive%20Component%20Object%20Reference) (OtherActor :type Actor%20Object%20Reference) (OtherComp :type Primitive%20Component%20Object%20Reference) (OtherBodyIndex :type Integer) (bFromSweep :type Boolean) (SweepResult :type Hit%20Result%20Structure%20%28by%20ref%29))
  (if (== OtherActor (Variables|Default|GetPlayer))
    (if (not (Variables|Default|GetAlreadyHitPlayer))
      (Development|PrintString (Utilities|GetDisplayName OtherActor))
      (Variables|Default|SetAlreadyHitPlayer true)
      (Audio|Components|Audio|FadeOut (Variables|Default|GetSoundSource) 2.0 0.0 "Linear" :!class /Script/Engine.AudioComponent)
      (Default|NextWayPointStart (Variables|Default|GetWaypointManager))
      (Audio|Components|Audio|StopDelayed (Variables|Default|GetSoundSource) 3.0)
      (Rendering|SetActorHiddenInGame true))))

(event EventBeginPlay
  (bind _asfirst_person_character (Utilities|Casting|CastToFirstPersonCharacter (Game|Player|GetPlayerPawn 0)))
  (Variables|Default|SetPlayer _asfirst_person_character)
  (bind _returnvalue (Actor|GetActorOfClass "/Game/Labyrinth/Blueprints/WaypointManagement_BP.WaypointManagement_BP_C"))
  (Variables|Default|SetWaypointManager _returnvalue))

(fn ConstructionScript)

(fn PlayMusic
  (Audio|Components|Audio|Play (Variables|Default|GetSoundSource) 0.0))