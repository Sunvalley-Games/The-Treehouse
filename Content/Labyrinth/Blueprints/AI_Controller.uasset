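; AI controller that makes the Labyrinth dinosaur chase the player and grow faster over time.
; After a short delay at start, it caches the LocomotionPawn_Final player and issues one move-to-actor toward it.
; A looping timer then has the Dino_BP pawn roar, call its speed-up step and gain max walk speed, with interval and increment set in the construction script.
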(event Custom|IncreaseSpeed
  (bind _asdino_bp (Utilities|Casting|CastToDino_BP (Pawn|GetControlledPawn)))
  (Default|PlayRoar _asdino_bp)
  (Default|SpeedUpStep _asdino_bp)
  (Variables|/Script/Engine.CharacterMovementComponent|SetMaxWalkSpeed (Variables|/Script/Engine.Character|GetCharacterMovement _asdino_bp) (+ (Class|MovementComponent|GetMaxSpeed (Variables|/Script/Engine.Character|GetCharacterMovement _asdino_bp)) (Variables|Default|GetSpeedIncrease))))

(event EventBeginPlay
  (Utilities|FlowControl|Delay 1.0)
  (bind _aslocomotion_pawn_final (Utilities|Casting|CastToLocomotionPawn_Final (Game|Player|GetPlayerPawn 0)))
  (bind _output_get (Variables|Default|SetPlayer _aslocomotion_pawn_final))
  (AI|Navigation|MovetoActor _output_get -1.0 true true true 0)
  (Utilities|Time|SetTimerbyEvent (delegate Custom|IncreaseSpeed) (Variables|Default|GetSpeedTime) true))

(fn ConstructionScript
  (Variables|Default|SetSpeedTime 15.0)
  (Variables|Default|SetSpeedIncrease 6e+01))