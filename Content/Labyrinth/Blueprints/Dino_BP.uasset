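; Dinosaur threat for the Labyrinth game that ends the run when it touches the VR player.
; On begin play it caches the LocomotionPawn_Final player and starts its looping-role step and roar sounds, with SpeedUpStep raising the step pitch on each call.
; A capsule overlap with that player, gated by HitPlayer, pauses the game and shows the Gameover widget.
; A separate Gameover event loads LevelToLoad once.
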(event OnComponentBeginOverlap(CapsuleComponent)
  (params (OverlappedComponent :type Primitive%20Component%20Object%20Reference) (OtherActor :type Actor%20Object%20Reference) (OtherComp :type Primitive%20Component%20Object%20Reference) (OtherBodyIndex :type Integer) (bFromSweep :type Boolean) (SweepResult :type Hit%20Result%20Structure%20%28by%20ref%29))
  (if (== OtherActor (Variables|Default|GetPlayerVR))
    (if (Variables|Default|GetHitPlayer)
      (Variables|Default|SetHitPlayer false)
      (Development|PrintString "Gameover" true true "(R=1.000000,G=0.028798,B=0.000000,A=1.000000)" 4.0)
      (Game|SetGamePaused true)
      (bind _returnvalue (UserInterface|CreateWidget "/Game/Labyrinth/Blueprints/Gameover.Gameover_C"))
      (UserInterface|Viewport|AddtoViewport _returnvalue 0))))

(event OnComponentBeginOverlap(Box)
  (params (OverlappedComponent :type Primitive%20Component%20Object%20Reference) (OtherActor :type Actor%20Object%20Reference) (OtherComp :type Primitive%20Component%20Object%20Reference) (OtherBodyIndex :type Integer) (bFromSweep :type Boolean) (SweepResult :type Hit%20Result%20Structure%20%28by%20ref%29)))

(event Custom|Gameover
  ;[1 1 1] gameover event
  (Development|PrintString "In gameover")
  (Utilities|FlowControl|DoOnce false
    (:Completed
      (Game|OpenLevel(byName) (Variables|Default|GetLevelToLoad)))))

(event EventBeginPlay
  ;[1 1 1] Event Begin Play
  (bind _aslocomotion_pawn_final (Utilities|Casting|CastToLocomotionPawn_Final (Game|Player|GetPlayerPawn 0)))
  (Variables|Default|SetPlayerVR _aslocomotion_pawn_final)
  (Audio|Components|Audio|Play (Variables|Default|GetSoundSource) 0.0)
  (CallFunction|PlayRoar))

(fn ConstructionScript)

(fn PlayRoar
  (Audio|Components|Audio|Play (Variables|Default|GetSoundSorceRoar) 0.0))

(fn SpeedUpStep
  (bind _result (Math|Float|IncrementFloat (Variables|Default|GetSoundPitch))
    (:%20%20
      (Audio|Components|Audio|SetPitchMultiplier (Variables|Default|GetSoundSource) _result))))