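; WaypointManagement_BP steps through an ordered Waypoints array in the labyrinth, starting music on one waypoint at a time.
; On BeginPlay it resets CurrentPoint to the first entry and calls PlayMusic on that waypoint.
; NextWayPointStart increments the index, casts that entry to Waypoint_BP and plays its music, with no array bounds check or call to stop the previous waypoint.
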(event EventBeginPlay
  (Variables|Default|SetCurrentPoint 0)
  (Default|PlayMusic (Utilities|Array|Get(acopy) (Variables|Default|GetWaypoints) (Variables|Default|GetCurrentPoint))))

(fn ConstructionScript)

(fn NextWayPointStart
  (bind _output_get (Variables|Default|SetCurrentPoint (+ (Variables|Default|GetCurrentPoint) 1)))
  (bind _aswaypoint_bp (Utilities|Casting|CastToWaypoint_BP (Utilities|Array|Get(acopy) (Variables|Default|GetWaypoints) _output_get)))
  (Default|PlayMusic _aswaypoint_bp))