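; FakeEnemy Blueprint that ends the game when the player touches its Box collider.
; BeginPlay caches the FirstPersonCharacter pawn; the first overlap with it sets a hit flag, pauses the game and shows the Gameover widget.
; A separate Gameover event opens LevelToLoad once through a DoOnce, but nothing in this file calls it.
; Debug prints remain, along with an unused LocomotionPawn_Final cast.
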(event OnComponentBeginOverlap(Box)
  (params (OverlappedComponent :type Primitive%20Component%20Object%20Reference) (OtherActor :type Actor%20Object%20Reference) (OtherComp :type Primitive%20Component%20Object%20Reference) (OtherBodyIndex :type Integer) (bFromSweep :type Boolean) (SweepResult :type Hit%20Result%20Structure%20%28by%20ref%29))
  (if (== OtherActor (Variables|Default|GetPlayer))
    (if (not (Variables|Default|GetHitplayer))
      (Variables|Default|SetHitplayer true)
      (Development|PrintString "Gameover" true true "(R=1.000000,G=0.028798,B=0.000000,A=1.000000)" 4.0)
      (Game|SetGamePaused true)
      (bind _returnvalue (UserInterface|CreateWidget "/Game/Labyrinth/Blueprints/Gameover.Gameover_C"))
      (UserInterface|Viewport|AddtoViewport _returnvalue 0))))

(event Custom|Gameover
  ;[1 1 1] gameover event
  (Development|PrintString "In gameover")
  (Utilities|FlowControl|DoOnce false
    (:Completed
      (Game|OpenLevel(byName) (Variables|Default|GetLevelToLoad)))))

(event EventBeginPlay
  ;[1 1 1] Event Begin Play
  (bind _asfirst_person_character (Utilities|Casting|CastToFirstPersonCharacter (Game|Player|GetPlayerPawn 0)))
  (bind _output_get (Variables|Default|SetPlayer _asfirst_person_character))
  (Development|PrintString (Utilities|GetDisplayName _output_get) true true "(R=0.000000,G=0.660000,B=1.000000,A=1.000000)" 3.0))

(fn ConstructionScript)