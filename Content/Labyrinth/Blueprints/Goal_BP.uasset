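; Labyrinth goal actor that handles the player's arrival with fireworks and audio, and destroys the enemy on contact.
; BeginPlay caches the LocomotionPawn_Final player and silences the audio.
; PlayerEnterGoal, not called within this Blueprint, unhides the Firework actors, then enables the Block's box collision and plays audio.
; Mesh overlap destroys the Enemy reference, while SetEnemy stores the found Dino_BP in a separate EnemyVR variable.
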(event OnComponentBeginOverlap(StaticMeshComponent)
  (params (OverlappedComponent :type Primitive%20Component%20Object%20Reference) (OtherActor :type Actor%20Object%20Reference) (OtherComp :type Primitive%20Component%20Object%20Reference) (OtherBodyIndex :type Integer) (bFromSweep :type Boolean) (SweepResult :type Hit%20Result%20Structure%20%28by%20ref%29))
  (bind _enemy (Variables|Default|GetEnemy))
  (if (and (== OtherActor _enemy) (Utilities|IsValid _enemy))
    (Actor|DestroyActor (Variables|Default|GetEnemy))))

(event EventBeginPlay
  (bind _aslocomotion_pawn_final (Utilities|Casting|CastToLocomotionPawn_Final (Game|Player|GetPlayerPawn 0)))
  (Variables|Default|SetPlayerVr _aslocomotion_pawn_final)
  (Audio|Components|Audio|Stop (Variables|Default|GetAudio)))

(fn ConstructionScript)

(fn SetEnemy
  (bind _returnvalue (Actor|GetActorOfClass "/Game/Labyrinth/Blueprints/Dino_BP.Dino_BP_C"))
  (Variables|Default|SetEnemyVR _returnvalue))

(fn PlayerEnterGoal
  (bind _firework (Variables|Default|GetFirework))
  (bind _block (Variables|Default|GetBlock))
  (if (Utilities|Array|IsValidIndex _firework)
    (for _array_element _firework
      (Rendering|SetActorHiddenInGame _array_element false))
    (if (Utilities|IsValid _block)
      (Collision|SetCollisionEnabled (Variables|/Game/Labyrinth/Blueprints/CubeToBlockAfterPlayerEnterWinning_BP.CubeToBlockAfterPlayerEnterWinning_BP_C|GetBox _block) "QueryAndPhysics")
      (Audio|Components|Audio|Play (Variables|Default|GetAudio) 0.0))))