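; Labyrinth goal actor that destroys the enemy when it overlaps the goal mesh and provides the response to the player reaching the goal.
; BeginPlay caches the first-person player, while a separate SetEnemy function finds the PrototypeEnemy_Blueprint instance to match against overlaps.
; PlayerEnterGoal, not called within this Blueprint, prints a debug message, unhides the Firework actors and enables collision on the Block's box.
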(event OnComponentBeginOverlap(StaticMeshComponent)
  (params (OverlappedComponent :type Primitive%20Component%20Object%20Reference) (OtherActor :type Actor%20Object%20Reference) (OtherComp :type Primitive%20Component%20Object%20Reference) (OtherBodyIndex :type Integer) (bFromSweep :type Boolean) (SweepResult :type Hit%20Result%20Structure%20%28by%20ref%29))
  (bind _enemy (Variables|Default|GetEnemy))
  (if (and (== OtherActor _enemy) (Utilities|IsValid _enemy))
    (Actor|DestroyActor (Variables|Default|GetEnemy))))

(event EventBeginPlay
  (bind _asfirst_person_character (Utilities|Casting|CastToFirstPersonCharacter (Game|Player|GetPlayerPawn 0)))
  (Variables|Default|SetPlayer _asfirst_person_character))

(fn ConstructionScript)

(fn SetEnemy
  (bind _returnvalue (Actor|GetActorOfClass "/Game/Labyrinth/Blueprints/PrototypeEnemy_Blueprint.PrototypeEnemy_Blueprint_C"))
  (Variables|Default|SetEnemy _returnvalue))

(fn PlayerEnterGoal
  (bind _firework (Variables|Default|GetFirework))
  (bind _block (Variables|Default|GetBlock))
  (Development|PrintString "TryingPlayer" true true "(R=0.000000,G=0.660000,B=1.000000,A=1.000000)" 4.0)
  (if (Utilities|Array|IsValidIndex _firework)
    (for _array_element _firework
      (Rendering|SetActorHiddenInGame _array_element false)
      (if (Utilities|IsValid _block)
        (Collision|SetCollisionEnabled (Variables|/Game/Labyrinth/Blueprints/CubeToBlockAfterPlayerEnterWinning_BP.CubeToBlockAfterPlayerEnterWinning_BP_C|GetBox _block) "QueryAndPhysics")))))